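; Player controller for the platform mode that owns the HUD and tracks the player's health.
; On BeginPlay it creates and adds the score and health bar widgets to the viewport, keeping a reference to the health bar.
; Its OnHitPlayer event subtracts a fixed amount of Hp and pushes the new health fraction to the health bar.
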(event Custom|OnHitPlayer
  (Variables|Default|Sethp (- (Variables|Default|Gethp) 5.0))
  (Default|UpdateUI (Variables|Default|GetHealthBarUI) (/ (Variables|Default|Gethp) (Variables|Default|GethpMax))))

(event EventBeginPlay
  (bind _returnvalue (UserInterface|CreateWidget "/Game/Blueprints/Platform/WBP_ScorePlatform.WBP_ScorePlatform_C"))
  (UserInterface|Viewport|AddtoViewport _returnvalue 0)
  (bind _returnvalue_2 (UserInterface|CreateWidget "/Game/Blueprints/Platform/WBP_HealthBar.WBP_HealthBar_C"))
  (bind _output_get (Variables|Default|SetHealthBarUI _returnvalue_2))
  (UserInterface|Viewport|AddtoViewport _output_get 0))

(fn ConstructionScript)