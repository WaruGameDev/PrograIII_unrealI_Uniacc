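; Player character for a 2D side-view platformer, moving along the world Y axis with a flipbook sprite.
; On BeginPlay it adds the platform input mapping context, and Enhanced Input actions drive horizontal movement and jumping.
; Each tick, movement velocity and falling state select the idle, run, jump or fall flipbook.
; The sprite rotates 180 degrees to face the travel direction, keeping its last facing when stationary.
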(event Input|EnhancedActionEvents|EnhancedInputActionIA_PlatformMove
  (params (ActionValue :type Float%20%28double-precision%29) (ElapsedSeconds :type Float%20%28double-precision%29) (TriggeredSeconds :type Float%20%28double-precision%29) (InputAction :type Input%20Action%20Object%20Reference :default "/Game/Input/Platform/IA_PlatformMove.IA_PlatformMove"))
  (Pawn|Input|AddMovementInput (Math|Vector|MakeVector 0.0 ActionValue 0.0) 1.0 false))

(event Input|EnhancedActionEvents|EnhancedInputActionIA_JumpPlatform
  (params (ActionValue :type Boolean) (ElapsedSeconds :type Float%20%28double-precision%29) (TriggeredSeconds :type Float%20%28double-precision%29) (InputAction :type Input%20Action%20Object%20Reference :default "/Game/Input/Platform/IA_JumpPlatform.IA_JumpPlatform"))
  (Character|Jump))

(event EventBeginPlay
  (bind _asbp_player_controller_platform (Utilities|Casting|CastToBP_PlayerControllerPlatform (Game|GetPlayerController 0)))
  (Input|AddMappingContext (PlayerController|LocalPlayerSubsystems|GetEnhancedInputLocalPlayerSubsystem _asbp_player_controller_platform) "/Game/Input/Platform/IMC_PlatformController.IMC_PlatformController" 0 "(bIgnoreAllPressedKeysUntilRelease=True,bForceImmediately=False,bNotifyUserSettings=False)"))

(event EventTick
  (params (DeltaSeconds :type Float%20%28single-precision%29))
  (CallFunction|SetAnimarion)
  (CallFunction|SetRotation))

(fn ConstructionScript)

(fn SetAnimarion
  (bind _charactermovement (Variables|Character|GetCharacterMovement))
  (bind _flippbookcharacter (Variables|Default|GetFlippbookCharacter))
  (bind _flippbookcharacter_2 (Variables|Default|GetFlippbookCharacter))
  (if (AI|Components|NavMovement|IsFalling _charactermovement)
    (if (> (.z (Variables|/Script/Engine.MovementComponent|GetVelocity _charactermovement)) 0.0)
      (Sprite|SetFlipbook _flippbookcharacter "/Game/Sprites/ranita/FB_jump.FB_jump")
      (else
        (Sprite|SetFlipbook _flippbookcharacter "/Game/Sprites/ranita/FB_Fall.FB_Fall")))
    (elif (> (Math|Float|Absolute(Float) (.y (Variables|/Script/Engine.MovementComponent|GetVelocity (Variables|Character|GetCharacterMovement)))) 0.0)
      (Sprite|SetFlipbook _flippbookcharacter_2 "/Game/Sprites/ranita/FB_Run.FB_Run")
      (else
        (Sprite|SetFlipbook _flippbookcharacter_2 "/Game/Sprites/ranita/FB_Idle.FB_Idle")))))

(fn SetRotation
  (bind _charactermovement (Variables|Character|GetCharacterMovement))
  (bind _flippbookcharacter (Variables|Default|GetFlippbookCharacter))
  (bind _velocity (Variables|/Script/Engine.MovementComponent|GetVelocity _charactermovement))
  (if (!= (.y _velocity) 0.0)
    (if (< (.y _velocity) 0.0)
      (Transformation|SetRelativeRotation _flippbookcharacter "0.000000,180.000000,0.000000" false false)
      (else
        (Transformation|SetRelativeRotation _flippbookcharacter "0.000000,0.000000,0.000000" false false)))))